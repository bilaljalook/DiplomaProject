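; Player projectile actor that kills horde enemies when its paper sprite overlaps them, then destroys itself.
; Each kill adds to the player's kills and points, lowers the wave game mode's enemy count and copies both stats into its save variables.
; The Hit event joins the same destroy chain without its own cast, while an Enemy_AI_BP cast branch is left disconnected.
; The construction script doubles the actor's scale.
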(event OnComponentBeginOverlap(PaperSprite)
  (params (OverlappedComponent :type Primitive%20Component%20Object%20Reference) (OtherActor :type Actor%20Object%20Reference) (OtherComp :type Primitive%20Component%20Object%20Reference) (OtherBodyIndex :type Integer) (bFromSweep :type Boolean) (SweepResult :type Hit%20Result%20Structure%20%28by%20ref%29))
  ;[1 1 1] Projectile kills
  (bind _ashorde_enemy_bp (Utilities|Casting|CastToHordeEnemy_BP OtherActor))
  (Actor|DestroyActor (stale _asenemy_ai_bp))
  ;[1 1 1] Stats for the player
  (Actor|DestroyActor)
  (bind _asplayer_bp (Utilities|Casting|CastToPlayerBP (Game|GetPlayerCharacter 0)))
  (bind _output_get (Variables|/Game/Blueprints/Players/PlayerBP.PlayerBP_C|SetKills _asplayer_bp (+ (Variables|/Game/Blueprints/Players/PlayerBP.PlayerBP_C|GetKills _asplayer_bp) 1)))
  (bind _output_get_2 (Variables|/Game/Blueprints/Players/PlayerBP.PlayerBP_C|SetPoints _asplayer_bp (+ (Variables|/Game/Blueprints/Players/PlayerBP.PlayerBP_C|GetPoints _asplayer_bp) 85)))
  (bind _asgame_mode_wave_system (Utilities|Casting|CastToGameMode_WaveSystem (Game|GetGameMode)))
  (Variables|/Game/Blueprints/ControllersAndGameModes/GameMode_WaveSystem.GameMode_WaveSystem_C|SetEnemyCount _asgame_mode_wave_system (- (Variables|/Game/Blueprints/ControllersAndGameModes/GameMode_WaveSystem.GameMode_WaveSystem_C|GetEnemyCount _asgame_mode_wave_system) 1))
  (Utilities|Casting|CastToPlayerBP (Game|GetPlayerCharacter 0))
  (Variables|/Game/Blueprints/ControllersAndGameModes/GameMode_WaveSystem.GameMode_WaveSystem_C|SetSavePoints _asgame_mode_wave_system _output_get_2)
  (Variables|/Game/Blueprints/ControllersAndGameModes/GameMode_WaveSystem.GameMode_WaveSystem_C|SetSaveKills _asgame_mode_wave_system _output_get))

(event Collision|EventHit
  (params (MyComp :type Primitive%20Component%20Object%20Reference) (Other :type Actor%20Object%20Reference) (OtherComp :type Primitive%20Component%20Object%20Reference) (bSelfMoved :type Boolean) (HitLocation :type Vector :default "0, 0, 0") (HitNormal :type Vector :default "0, 0, 0") (NormalImpulse :type Vector :default "0, 0, 0") (Hit :type Hit%20Result%20Structure%20%28by%20ref%29))
  ;[1 1 1] Projectile kills
  (Actor|DestroyActor (stale _asenemy_ai_bp))
  ;[1 1 1] Stats for the player
  (Actor|DestroyActor)
  (bind _asplayer_bp (Utilities|Casting|CastToPlayerBP (Game|GetPlayerCharacter 0)))
  (bind _output_get (Variables|/Game/Blueprints/Players/PlayerBP.PlayerBP_C|SetKills _asplayer_bp (+ (Variables|/Game/Blueprints/Players/PlayerBP.PlayerBP_C|GetKills _asplayer_bp) 1)))
  (bind _output_get_2 (Variables|/Game/Blueprints/Players/PlayerBP.PlayerBP_C|SetPoints _asplayer_bp (+ (Variables|/Game/Blueprints/Players/PlayerBP.PlayerBP_C|GetPoints _asplayer_bp) 85)))
  (bind _asgame_mode_wave_system (Utilities|Casting|CastToGameMode_WaveSystem (Game|GetGameMode)))
  (Variables|/Game/Blueprints/ControllersAndGameModes/GameMode_WaveSystem.GameMode_WaveSystem_C|SetEnemyCount _asgame_mode_wave_system (- (Variables|/Game/Blueprints/ControllersAndGameModes/GameMode_WaveSystem.GameMode_WaveSystem_C|GetEnemyCount _asgame_mode_wave_system) 1))
  (Utilities|Casting|CastToPlayerBP (Game|GetPlayerCharacter 0))
  (Variables|/Game/Blueprints/ControllersAndGameModes/GameMode_WaveSystem.GameMode_WaveSystem_C|SetSavePoints _asgame_mode_wave_system _output_get_2)
  (Variables|/Game/Blueprints/ControllersAndGameModes/GameMode_WaveSystem.GameMode_WaveSystem_C|SetSaveKills _asgame_mode_wave_system _output_get))

(fn ConstructionScript
  (Transformation|SetActorScale3D "2.000000,2.000000,2.000000"))