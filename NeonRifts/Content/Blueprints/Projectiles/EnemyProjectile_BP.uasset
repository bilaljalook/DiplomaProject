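; Enemy projectile actor that carries damage to whatever its Bullet component hits and expires after ten seconds.
; SetDamageInfo stores the damage range and crit chance on the projectile.
; On hit it sends those values, bone name and instigator to actors implementing DamageInterface_BP via TickDamageMessage, then always destroys itself.
; The impact sound plays at world origin, as no hit or actor location is wired in.
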(event `self.ReceiveBeginPlay`
  (`self.SetLifeSpan` 10.0))

(event `self.Bullet.OnComponentHit`
  (params (HitComponent :type "PrimitiveComponent Object Reference") (OtherActor :type "Actor Object Reference") (OtherComp :type "PrimitiveComponent Object Reference") (NormalImpulse :type "Vector Structure") (Hit :type "HitResult Structure (by ref)"))
  (bind (_bblockinghit _binitialoverlap _time _location _impactpoint _normal _impactnormal _physmat _hitactor _hitcomponent _hitbonename) (`GameplayStatics.BreakHitResult` Hit))
  (`GameplayStatics.PlaySoundAtLocation` (`self.ImpactSound`))
  (if (`KismetSystemLibrary.DoesImplementInterface` _hitactor "/Game/Blueprints/Enemy_AI/DamageInterface_BP.DamageInterface_BP_C")
    (message `/Game/Blueprints/Enemy_AI/DamageInterface_BP.TickDamage` _hitactor (`self.DamageMin`) (`self.DamageMax`) (`self.CritChance`) _hitbonename (`self.GetInstigator`))
    (`self.K2_DestroyActor`)
    (else
      (`self.K2_DestroyActor`))))

(fn `SetDamageInfo`
  (params (DamageMin :type "Float (double-precision)") (DamageMax :type "Float (double-precision)") (CritChance :type "Float (double-precision)"))
  (set `self.DamageMin` DamageMin)
  (set `self.DamageMax` DamageMax)
  (set `self.CritChance` CritChance))

(fn `UserConstructionScript`)