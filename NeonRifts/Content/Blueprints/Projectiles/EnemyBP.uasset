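; EnemyBP is a 2D sprite enemy that moves along two waypoints and hurts the player on contact.
; The construction script feeds relative PointA and PointB into InterpToMovement as control points.
; Box overlap launches PlayerBP using the hit normal and an upward kick, then applies damage.
; ShootEnemy is unfinished, only spawning an emitter and tracing without using the result, while sprite flipping and delayed destruction are disconnected.
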(event `self.ReceiveBeginPlay`)

(event `self.InterpToMovement.OnInterpToReverse`
  (params (ImpactResult :type "HitResult Structure (by ref)") (Time :type "Float (single-precision)"))
  ;[1 1 1] rotating the character's sprite
)

(event `self.Box.OnComponentBeginOverlap`
  (params (OverlappedComponent :type "PrimitiveComponent Object Reference") (OtherActor :type "Actor Object Reference") (OtherComp :type "PrimitiveComponent Object Reference") (OtherBodyIndex :type Integer) (bFromSweep :type Boolean) (SweepResult :type "HitResult Structure (by ref)"))
  ;[1 1 1] aftereffect from damage recieved
  (bind _asplayer_bp (cast `/Game/Blueprints/Players/PlayerBP` OtherActor))
  (`Character.LaunchCharacter` _asplayer_bp (`KismetMathLibrary.MakeVector` (* (.x (`.Normal` (`GameplayStatics.BreakHitResult` SweepResult))) -400.0) 0.0 200.0) true true)
  (`GameplayStatics.ApplyDamage` _asplayer_bp 10.0 null null "/Script/Engine.DamageType"))

(event `ShootEnemy`
  (params (EnemyToShoot :type "Actor Object Reference"))
  ;[1 1 1] WIP
  (`self.PlayShootFX`)
  (`KismetSystemLibrary.LineTraceSingle` (`self.K2_GetActorLocation`) (`self.K2_GetActorLocation` EnemyToShoot) "TraceTypeQuery1"))

(event `PlayShootFX`
  ;[1 1 1] WIP
  (`GameplayStatics.SpawnEmitterAtLocation` null))

(fn `UserConstructionScript`
  ;[1 1 1] Waypoints
  (set `InterpToMovementComponent.ControlPoints` (`|MakeArray` (make `InterpControlPoint` (`self.PointA`)) (make `InterpControlPoint` (`self.PointB`))) (`self.InterpToMovement`)))