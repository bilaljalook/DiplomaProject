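; Projectile Blueprint that destroys enemies of type Enemy_AI_BP on sprite overlap, then destroys itself.
; Overlap casts the other actor to Enemy_AI_BP; the failed-cast branch and the Hit event share a destroy call on that cast result rather than on the actor struck.
; Damage and collision-disabling nodes are disconnected and never run.
; The construction script doubles the actor's scale.
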(event `self.PaperSprite.OnComponentBeginOverlap`
  (params (OverlappedComponent :type "PrimitiveComponent Object Reference") (OtherActor :type "Actor Object Reference") (OtherComp :type "PrimitiveComponent Object Reference") (OtherBodyIndex :type Integer) (bFromSweep :type Boolean) (SweepResult :type "HitResult Structure (by ref)"))
  (bind _asenemy_ai_bp (cast `/Game/Blueprints/Players/Enemy_AI_BP` OtherActor)
    (:`then`
      (`self.K2_DestroyActor` _asenemy_ai_bp))
    (:`CastFailed`
      (`self.K2_DestroyActor` _asenemy_ai_bp :!label _label)))
  (`self.K2_DestroyActor`))

(event `self.ReceiveHit`
  (params (MyComp :type "PrimitiveComponent Object Reference") (Other :type "Actor Object Reference") (OtherComp :type "PrimitiveComponent Object Reference") (bSelfMoved :type Boolean) (HitLocation :type "Vector Structure") (HitNormal :type "Vector Structure") (NormalImpulse :type "Vector Structure") (Hit :type "HitResult Structure (by ref)"))
  (goto _label))

(fn `UserConstructionScript`
  (`self.SetActorScale3D` (2.0 2.0 2.0)))