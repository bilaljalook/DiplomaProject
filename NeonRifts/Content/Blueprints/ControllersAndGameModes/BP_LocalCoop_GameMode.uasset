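; Local co-op game mode that creates the local players and spawns their characters when play begins.
; It gathers all PlayerStart actors, then for each index up to MaxPlayerCount finds starts whose PlayerStartTag matches that index.
; At a match it creates the local player, spawns a pawn there and has that player's controller possess it.
; Player 0 gets PlayerBP, while the other players get BP_PaperCharacter.
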(event `self.ReceiveBeginPlay`
  (`self.GetPlayersStartPoints`)
  (`self.SpawnPlayers`))

(fn `GetPlayersStartPoints`
  (bind _outactors (`GameplayStatics.GetAllActorsOfClass` "/Script/Engine.PlayerStart"))
  (set `self.PlayerStartArray` _outactors))

(fn `SpawnPlayers`
  (bind _index (`self.Index`))
  (bind _returnvalue (`GameplayStatics.GetPlayerController` (`self.Index`)))
  (for _index_2 (range (`self.MaxPlayerCount`))
    (set `self.Index` _index_2)
    (for _array_element (`self.PlayerStartArray`)
      (if (== (`PlayerStart.PlayerStartTag` _array_element) (`KismetStringLibrary.Conv_StringToName` (`KismetStringLibrary.Conv_IntToString` (`self.Index`))))
        (if (== (`self.Index`) 0)
          (`GameplayStatics.CreatePlayer` _index)
          (bind _returnvalue_2 (`self.GetTransform` _array_element))
          (bind _returnvalue_3 (`|SpawnActorFromClass` "/Game/Blueprints/Players/PlayerBP.PlayerBP_C" _returnvalue_2 "AlwaysSpawn" "OverrideRootScale" null null))
          (`Controller.Possess` _returnvalue _returnvalue_3)
          (else
            (`GameplayStatics.CreatePlayer` _index)
            (bind _returnvalue_4 (`|SpawnActorFromClass` "/Game/Blueprints/Players/BP_PaperCharacter.BP_PaperCharacter_C" _returnvalue_2 "AlwaysSpawn" "OverrideRootScale" null null))
            (`Controller.Possess` _returnvalue _returnvalue_4)))
        (`KismetArrayLibrary.Array_AddUnique` (`self.Players`))))))

(fn `UserConstructionScript`)