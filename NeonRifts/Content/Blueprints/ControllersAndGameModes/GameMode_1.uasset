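; Game mode that runs an enemy horde wave system, starting once after an initial delay.
; Each wave increments the wave number, grows the enemy count and spawns HordeEnemy_BP at random WaveSpawner actors.
; A Delay loop polls EnemyCount; at zero it updates the player's waves survived and waits before the next wave.
; A work-in-progress Tick timer counts down the break, and UpdateEnemyAttributes is called on the first enemy found.
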(event `self.ReceiveTick`
  (params (DeltaSeconds :type "Float (single-precision)"))
  ;[1 1 1] SpawnSystem
  ;;[1 1 1] Timer  (WIP)
  (`KismetSystemLibrary.Delay` 1.0)
  (set `self.TimeBetweenWaves` (- (`self.TimeBetweenWaves`) 1.0))
  (if (== (`self.TimeBetweenWaves`) 0.0)
    (set `self.IsTimeBetweenWaves` false)))

(event `Start`
  ;[1 1 1] SpawnSystem
  ;;[1 1 1] Start the Wave
  (`/Engine/EditorBlueprintResources/StandardMacros.DoOnce` false
    (:`Completed`
      (set `self.GameStarted` true) ; game is started
      (`KismetSystemLibrary.Delay` (`self.GameStartTime`)) ; game start time
      (`self.Wave`))))

(event `StartTimer`
  ;[1 1 1] SpawnSystem
  ;;[1 1 1] Timer  (WIP)
)

(event `StopTimer`
  ;[1 1 1] SpawnSystem
  ;;[1 1 1] Timer  (WIP)
)

(event `Wave`
  (bind _timebetweenwaves (`self.TimeBetweenWaves`))
  (bind _enemystartcount (`self.EnemyStartCount`))
  ;[1 1 1] SpawnSystem
  ;;[1 1 1] waves
  (`self.updatewave`)
  (set `self.TimeBetweenWaves` 8.0)
  (set `self.EnemyStartCount` (+ _enemystartcount (`self.EnemiesAddedEachWave`))) ; add more enemies on every wave
  (for _index (range 1 (+ _enemystartcount 1))
    (bind _outactors (`GameplayStatics.GetAllActorsOfClass` "/Game/Blueprints/WaveSystem/WaveSpawner.WaveSpawner_C"))
    (`|SpawnActorFromClass` "/Game/Blueprints/Players/HordeEnemy_BP.HordeEnemy_BP_C" (`self.GetTransform` (`|GetArrayItem` _outactors (`KismetMathLibrary.RandomIntegerInRange` 0 (`KismetArrayLibrary.Array_LastIndex` _outactors)))) "AdjustIfPossibleButAlwaysSpawn" "OverrideRootScale" null null) ; actor you want to spawn
    (bind _output_get (set `self.EnemyCount` _index))
    (if (<= _output_get 0) :!label _label
      (bind _asplayer_bp (cast `/Game/Blueprints/Players/PlayerBP` (`GameplayStatics.GetPlayerCharacter` 0)))
      (`/Game/Blueprints/Players/PlayerBP.UpdateWavesSurvived` _asplayer_bp)
      (`KismetSystemLibrary.Delay` 1.0)
      (set `self.TimeBetweenWaves` (- (`self.TimeBetweenWaves`) 1.0))
      (bind _output_get_2 (set `self.IsTimeBetweenWaves` true)) ; set waiting time on
      (set `self.TimeBetweenWaves` 8.0)
      (`KismetSystemLibrary.RetriggerableDelay` _timebetweenwaves)
      (if (== _timebetweenwaves 0.0)
        (set `self.IsTimeBetweenWaves` false) ; end waiting time
        (`self.Wave`)
        (bind _outactors_2 (`GameplayStatics.GetAllActorsOfClass` "/Game/Blueprints/Players/HordeEnemy_BP.HordeEnemy_BP_C"))
        (`/Game/Blueprints/Players/HordeEnemy_BP.UpdateEnemyAttributes` (`|GetArrayItem` _outactors_2)))
      (else
        (`KismetSystemLibrary.Delay` (`self.CheckSpeed`)) ; check enemies remain
        (goto _label)))))

(fn `UpdateWave`
  (set `self.WaveNumber` (+ (`self.WaveNumber`) 1)))

(fn `UserConstructionScript`)