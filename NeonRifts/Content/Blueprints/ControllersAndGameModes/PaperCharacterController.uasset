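; Player controller for paper characters that lets a player spawn and despawn their character at runtime.
; On BeginPlay it waits briefly, then creates a BP_HUD widget and stores it, without adding it to the viewport here.
; Keyboard 1/2 and gamepad Special Right/Left pass the controller to BP_PaperGameMode's SpawnCharacter and DespawnCharacter.
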(event `self.ReceiveBeginPlay`
  (`KismetSystemLibrary.Delay` 0.01)
  (bind _returnvalue (`|CreateWidget` "/Game/Blueprints/LocalCoop/BP_HUD.BP_HUD_C" self))
  (set `self.HUD` _returnvalue))

(event `Key|One`
  (params (Key :type "Key Structure"))
  (:`Pressed`
    (bind _asbp_paper_game_mode (cast `/Game/Blueprints/ControllersAndGameModes/BP_PaperGameMode` (`GameplayStatics.GetGameMode`) :!label _label))
    (`/Game/Blueprints/ControllersAndGameModes/BP_PaperGameMode.SpawnCharacter` _asbp_paper_game_mode self)))

(event `Key|Gamepad_Special_Right`
  (params (Key :type "Key Structure"))
  (:`Pressed`
    (goto _label)))

(event `Key|Gamepad_Special_Left`
  (params (Key :type "Key Structure"))
  (:`Pressed`
    (bind _asbp_paper_game_mode (cast `/Game/Blueprints/ControllersAndGameModes/BP_PaperGameMode` (`GameplayStatics.GetGameMode`) :!label _label_2))
    (`/Game/Blueprints/ControllersAndGameModes/BP_PaperGameMode.DespawnCharacter` _asbp_paper_game_mode self)))

(event `Key|Two`
  (params (Key :type "Key Structure"))
  (:`Pressed`
    (goto _label_2)))

(fn `UserConstructionScript`)