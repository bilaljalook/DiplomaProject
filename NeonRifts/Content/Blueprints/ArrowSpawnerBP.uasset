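; Arrow spawner actor that fires arrows while moving vertically from its starting position.
; On BeginPlay a looping one-second timer calls Fire, which spawns an ArrowBP at the SpawnPoint component's transform.
; A timeline drives a lerp between the start location and a Z offset given by MovingSpeed, which acts as a travel distance rather than a rate.
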(event `self.ReceiveBeginPlay`
  (bind (_startpos_x _startpos_y _startpos_z) (`KismetMathLibrary.BreakVector` (`self.StartPos`)))
  (set `self.StartPos` (`self.K2_GetActorLocation`))
  (`KismetSystemLibrary.K2_SetTimer` null "Fire" 1.0 true)
  (bind (_direction _movement) (`Timeline|MovementTimeline` :!via `PlayFromStart`)
    (:`Update`
      (`self.K2_SetActorLocation` (`KismetMathLibrary.VLerp` (`self.StartPos`) (`KismetMathLibrary.MakeVector` _startpos_x _startpos_y (+ _startpos_z (`self.MovingSpeed`))) _movement)))))

(event `Fire`
  (`|SpawnActorFromClass` "/Game/Blueprints/ArrowBP.ArrowBP_C" (`SceneComponent.K2_GetComponentToWorld` (`self.SpawnPoint`)) "Undefined" "OverrideRootScale" null null))

(fn `UserConstructionScript`)