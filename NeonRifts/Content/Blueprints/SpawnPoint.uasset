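; Spawn point actor that keeps a single AI unit of a configurable class alive in the level.
; BeginPlay and the Respawn event share one spawn path, which creates the AI at the actor's location and stores it as SpawnUnit.
; Tick polls that reference and, once it is invalid, waits for the respawn timer through a Delay before calling Respawn.
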(event `Respawn`
  (bind _returnvalue (`AIBlueprintHelperLibrary.SpawnAIFromClass` (`self.ClassToSpawn`) null (`self.K2_GetActorLocation`) :!label _label))
  (set `self.SpawnUnit` _returnvalue))

(event `self.ReceiveBeginPlay`
  (goto _label))

(event `self.ReceiveTick`
  (params (DeltaSeconds :type "Float (single-precision)"))
  (if (not (`KismetSystemLibrary.IsValid` (`self.SpawnUnit`)))
    (`KismetSystemLibrary.Delay` (`self.RespawnTimer`))
    (`self.Respawn`)))

(fn `UserConstructionScript`)