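; Enemy spawner actor that keeps feeding horde enemies into the level at random points inside its SpawnVolume box.
; BeginPlay starts a looping SpawnEnemy timer on the first EnemySpawner found in the world, not necessarily itself, with an interval of two divided by EnemiesPerSec.
; Each tick of that timer spawns a HordeEnemy_BP only while the count of Enemy_AI_BP actors is below MaxSpawnNum.
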(event `SpawnEnemy`
  (bind _spawnvolume (`self.SpawnVolume`))
  (bind _outactors (`GameplayStatics.GetAllActorsOfClass` "/Game/Blueprints/Players/Enemy_AI_BP.Enemy_AI_BP_C"))
  (if (< (`KismetArrayLibrary.Array_Length` _outactors) (`self.MaxSpawnNum`))
    (`AIBlueprintHelperLibrary.SpawnAIFromClass` "/Game/Blueprints/Players/HordeEnemy_BP.HordeEnemy_BP_C" null (`KismetMathLibrary.RandomPointInBoundingBox` (`SceneComponent.K2_GetComponentLocation` _spawnvolume) (`BoxComponent.GetScaledBoxExtent` _spawnvolume)))))

(event `self.ReceiveBeginPlay`
  (bind _outactors (`GameplayStatics.GetAllActorsOfClass` "EnemySpawner_C"))
  (bind _output (`|GetArrayItem` _outactors))
  (bind _output_get (set `/Game/Blueprints/EnemySpawner.Spawner` _output _output))
  (`KismetSystemLibrary.K2_SetTimer` _output_get "SpawnEnemy" (/ 2.0 (`self.EnemiesPerSec`)) true))

(fn `UserConstructionScript`)