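; Sprite-based enemy AI that switches to combat when PawnSensing sees or hears the player, and knocks back and damages the player on capsule contact.
; FireWeapon branches by combat type, but only Assault works, using a looping timer to spawn projectiles aimed at the player.
; TickDamage applies random damage with crits until death, while hits or player-projectile overlaps destroy it outright.
; Cover, Heavy and waypoint patrol are unfinished.
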(event `self.PawnSensing.OnSeePawn`
  (params (Pawn :type "Pawn Object Reference"))
  ;[1 1 1] PawnSensing
  (`self.SetToCombat` Pawn))

(event `IsCoverAvailable`
  (params (IsCoverAvailable :type Boolean) (CoverRot :type "Rotator Structure"))
  ;[1 1 1] Cover (WIP)
  (set `self.CoverAvailable` IsCoverAvailable)
  (set `self.CoverRot` CoverRot))

(event `self.ReceiveActorBeginOverlap`
  (params (OtherActor :type "Actor Object Reference"))
  (bind _asprojectile_player_bp (cast `/Game/Blueprints/Projectiles/ProjectilePlayer_BP` OtherActor))
  (`self.K2_DestroyActor` :!label _label)
  (`self.K2_DestroyActor` _asprojectile_player_bp))

(event `self.ReceiveHit`
  (params (MyComp :type "PrimitiveComponent Object Reference") (Other :type "Actor Object Reference") (OtherComp :type "PrimitiveComponent Object Reference") (bSelfMoved :type Boolean) (HitLocation :type "Vector Structure") (HitNormal :type "Vector Structure") (NormalImpulse :type "Vector Structure") (Hit :type "HitResult Structure (by ref)"))
  (goto _label))

(event `self.PawnSensing.OnHearNoise`
  (params (Instigator :type "Pawn Object Reference") (Location :type "Vector Structure (by ref)") (Volume :type "Float (single-precision)"))
  ;[1 1 1] PawnSensing
  (`self.SetToCombat` Instigator))

(event `self.ReceiveBeginPlay`
  (bind _sprite (`self.Sprite`))
  ;[1 1 1] Wayponts plus current health
  (set `self.Waypoint1` (`SceneComponent.K2_GetComponentLocation` (`self.WayPoint1BillBoard`)))
  (set `self.Waypoint2` (`SceneComponent.K2_GetComponentLocation` (`self.Waypoint2Billboard`)))
  ;[1 1 1] Rotation for Sprite
  (`/Engine/EditorBlueprintResources/StandardMacros.FlipFlop`
    (:`A`
      (`SceneComponent.K2_SetWorldRotation` :`self` _sprite) ; This is for Sprite, you change it,same name but for flipbook
    )
    (:`B`
      (`SceneComponent.K2_SetWorldRotation` _sprite (struct :`Yaw` 180.0) false false) ; This is for Sprite, you change it,same name but for flipbook
    )))

(event `/Game/Blueprints/Enemy_AI/DamageInterface_BP.TickDamage`
  (params (DamagMin :type "Float (single-precision)") (DamageMax :type "Float (single-precision)") (CritChance :type "Float (single-precision)") (HitBoneName :type Name) (DamageInstigator :type "Actor Object Reference"))
  ;[1 1 1] Event tick Damage
  (`|ExecutionSequence`
    (:`then_0`
      (`self.SetToCombat` DamageInstigator))
    (:`then_1`
      (`self.CalculateHealth` DamagMin DamageMax CritChance)
      (if (`self.IsDead`)
        (`self.K2_DestroyActor`)
        (`self.StopFireWeapon`)))))

(event `FireWeapon`
  ;[1 1 1] Fire
  (if (not (`self.IsDead`))
    (switch `/Game/Blueprints/Enemy_AI/CombatType_Enum` (`self.CombatType`)
      (:`NewEnumerator0`
        (`self.Assault`))
      (:`NewEnumerator1`
        (`self.Cover`))
      (:`NewEnumerator2`
        (`self.Heavy`)))))

(event `StopFireWeapon`
  ;[1 1 1] Fire
  (`KismetSystemLibrary.K2_ClearAndInvalidateTimerHandle` (`self.TimerHandle`)))

(event `Assault`
  ;[1 1 1] Fire
  (`self.FireAssault`)
  (bind _returnvalue (`KismetSystemLibrary.K2_SetTimerDelegate` (delegate `FireAssault`) 1.0 true))
  (set `self.TimerHandle` _returnvalue))

(event `self.CapsuleComponent.OnComponentBeginOverlap`
  (params (OverlappedComponent :type "PrimitiveComponent Object Reference") (OtherActor :type "Actor Object Reference") (OtherComp :type "PrimitiveComponent Object Reference") (OtherBodyIndex :type Integer) (bFromSweep :type Boolean) (SweepResult :type "HitResult Structure (by ref)"))
  ;[1 1 1] Melee Effect
  (bind _asplayer_bp (cast `/Game/Blueprints/Players/PlayerBP` OtherActor))
  (`self.LaunchCharacter` _asplayer_bp (`KismetMathLibrary.MakeVector` (* (.x (`.Normal` (`GameplayStatics.BreakHitResult` SweepResult))) -400.0) 0.0 200.0) false false)
  (`GameplayStatics.ApplyDamage` _asplayer_bp 10.0 null null "/Script/Engine.DamageType"))

(event `FireAssault`
  ;[1 1 1] Fire
  (if (< (`self.FireCount`) 5)
    (for _ (range 1 (+ (`self.FireBurst`) 1))
      (bind _projectilespawn (`self.CalculateFire`))
      (bind _returnvalue (`|SpawnActorFromClass` "/Game/Blueprints/Projectiles/ProjectileBP.ProjectileBP_C" _projectilespawn "Undefined" "OverrideRootScale" null self))
      (`GameplayStatics.ApplyDamage` _returnvalue 10.0 null null "/Script/Engine.DamageType"))
    (set `self.FireCount` (+ (`self.FireCount`) 1))
    (else
      (`KismetSystemLibrary.Delay` 1.0)
      (set `self.FireCount` 0))))

(event `Cover`)

(event `Heavy`)

(event `FireCover`
  ;[1 1 1] Fire-Differenet methods for different weapons(WIP)
)

(event `RifleB`
  ;[1 1 1] Fire-Differenet methods for different weapons(WIP)
)

(fn `CalculateFire`
  (returns (ProjectileSpawn :type "Transform Structure"))
  (return (`KismetMathLibrary.MakeTransform` (`SceneComponent.K2_GetComponentLocation` (`self.MuzzleArrow`)) (`KismetMathLibrary.FindLookAtRotation` (`self.K2_GetActorLocation`) (`self.K2_GetActorLocation` (`GameplayStatics.GetPlayerPawn` 0))))))

(fn `CalculateHealth`
  (params (DamageMin :type "Float (double-precision)") (DamageMax :type "Float (double-precision)") (CritChance :type "Float (double-precision)"))
  (locals (LocalDamage :type "Float (double-precision)" :default 0.0))
  (if (not (`self.IsDead`))
    (set `local.LocalDamage` (`KismetMathLibrary.Conv_IntToDouble` (`KismetMathLibrary.Round` (`KismetMathLibrary.RandomFloatInRange` DamageMin DamageMax))))
    (`|ExecutionSequence`
      (:`then_0`
        (if (<= (`KismetMathLibrary.RandomFloatInRange` 0.0 40.0) CritChance)
          (set `local.LocalDamage` (* (`local.LocalDamage`) 1.5))
          (`KismetSystemLibrary.PrintString` "Crit")))
      (:`then_1`
        (bind _output_get (set `self.CurrentHealth` (- (`self.CurrentHealth`) (`local.LocalDamage`))))
        (`KismetSystemLibrary.PrintString` (`KismetStringLibrary.Conv_DoubleToString` _output_get))
        (if (<= _output_get 0.0)
          (set `self.CurrentHealth` 0.0)
          (set `self.IsDead` true))))))

(fn `SetIsTakingCover`
  (params (IsTakingCover :type Boolean)))

(fn `SetToCombat`
  (params (SensedPawn :type "Object Object Reference"))
  (if (not (`|EnumEquality` (`self.CombatStatus`) "NewEnumerator2"))
    (bind _asplayer_bp (cast `/Game/Blueprints/Players/PlayerBP` SensedPawn))
    (set `self.PlayerCharacter` _asplayer_bp)
    (set `self.CombatStatus` "NewEnumerator2")))

(fn `UserConstructionScript`
  (`|ExecutionSequence`
    (:`then_0`
      (switch `/Game/Blueprints/Enemy_AI/CombatStatus_Enum` (`self.CombatStatus`)
        (:`NewEnumerator1`
          (`SceneComponent.SetVisibility` (`self.WayPoint1BillBoard`) true false)
          (`SceneComponent.SetVisibility` (`self.Waypoint2Billboard`) true false))))))