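; ExplodingEnemy_BP is a suicide-style enemy that runs at the player and destroys itself on contact.
; Pawn sensing triggers an AI move toward the player character.
; Capsule overlap with the player launches them using the hit normal, destroys the enemy and applies damage.
; Overlap with a player projectile destroys both actors, while the particle effect spawn is left unconnected.
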(event `self.PawnSensing.OnSeePawn`
  (params (Pawn :type "Pawn Object Reference"))
  ;[1 1 1] Run to player
  (bind _asplayer_bp (cast `/Game/Blueprints/Players/PlayerBP` (`GameplayStatics.GetPlayerCharacter` 0)))
  (`|AIMoveTo` self (0.0 0.0 0.0) _asplayer_bp 12.0))

(event `self.CapsuleComponent.OnComponentBeginOverlap`
  (params (OverlappedComponent :type "PrimitiveComponent Object Reference") (OtherActor :type "Actor Object Reference") (OtherComp :type "PrimitiveComponent Object Reference") (OtherBodyIndex :type Integer) (bFromSweep :type Boolean) (SweepResult :type "HitResult Structure (by ref)"))
  ;[1 1 1] After effect
  (bind _asplayer_bp (cast `/Game/Blueprints/Players/PlayerBP` OtherActor)
    (:`then`
      (`self.LaunchCharacter` _asplayer_bp (`KismetMathLibrary.MakeVector` (* (.x (`.Normal` (`GameplayStatics.BreakHitResult` SweepResult))) -400.0) 0.0 200.0) false false)
      (`self.K2_DestroyActor`)
      (`GameplayStatics.ApplyDamage` _asplayer_bp 10.0 null null "/Script/Engine.DamageType"))
    (:`CastFailed`
      ;[1 1 1] shot effect
      (bind _asprojectile_player_bp (cast `/Game/Blueprints/Projectiles/ProjectilePlayer_BP` OtherActor))
      (`self.K2_DestroyActor` _asprojectile_player_bp)
      (`self.K2_DestroyActor`))))

(event `self.CapsuleComponent.OnComponentHit`
  (params (HitComponent :type "PrimitiveComponent Object Reference") (OtherActor :type "Actor Object Reference") (OtherComp :type "PrimitiveComponent Object Reference") (NormalImpulse :type "Vector Structure") (Hit :type "HitResult Structure (by ref)"))
  ;[1 1 1] shot effect
)

(fn `UserConstructionScript`)