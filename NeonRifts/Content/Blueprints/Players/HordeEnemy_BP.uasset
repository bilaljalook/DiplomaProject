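; Wave-horde enemy character that chases the player and applies damage when within attack range.
; A self-restarting AIMoveTo loop drives it, re-randomizing walk speed and starting a short random nearby move after each hit.
; UpdateEnemyAttributes refreshes speed and sets damage from Wavedamage.
; Health, kill rewards, knockback, sprite flipping and roaming are unfinished or disconnected, so incoming damage has no effect.
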(event `self.CapsuleComponent.OnComponentBeginOverlap`
  (params (OverlappedComponent :type "PrimitiveComponent Object Reference") (OtherActor :type "Actor Object Reference") (OtherComp :type "PrimitiveComponent Object Reference") (OtherBodyIndex :type Integer) (bFromSweep :type Boolean) (SweepResult :type "HitResult Structure (by ref)"))
  ;[1 1 1] Melee effect
)

(event `self.ReceiveBeginPlay`
  ;[1 1 1] The Start
  (`self.Setstartspeed`)
  (`self.Chase/Attack again`))

(event `Chase/Attack again`
  ;[1 1 1] Chase and Attack
  (`|AIMoveTo` self (0.0 0.0 0.0) (`GameplayStatics.GetPlayerCharacter` 0) (`self.AttackLength`)
    (:`OnSuccess`
      ;[1 1 1] Check player health status
      (bind _asplayer_bp (cast `/Game/Blueprints/Players/PlayerBP` (`GameplayStatics.GetPlayerCharacter` 0)))
      (`GameplayStatics.ApplyDamage` _asplayer_bp (`self.EnemyDamage`) null null "/Script/Engine.DamageType")
      (`self.Chase/Attack again`)
      ;[1 1 1] distance and speed for attacking after the first attack
      (`self.UpdateEnemySpeed`)
      (`|AIMoveTo` self (`NavigationSystem.K2_GetRandomLocationInNavigableRadius` (`self.GetNavAgentLocation`) 10.0) null 11.0
        (:`OnSuccess`
          (`self.Chase/Attack again`))))
    (:`OnFail`
      (`self.Chase/Attack again`))))

(event `UpdateEnemyAttributes`
  ;[1 1 1] Update the enemy attributes
  (`self.UpdateEnemySpeed`)
  (`self.DamageOnWave`))

(event `PlayerStats`
  ;[1 1 1] Update stats to player (Not called, WIP)
  (bind _asplayer_bp (cast `/Game/Blueprints/Players/PlayerBP` (`GameplayStatics.GetPlayerCharacter` 0)))
  (set `/Game/Blueprints/Players/PlayerBP.Kills` (+ (`/Game/Blueprints/Players/PlayerBP.Kills` _asplayer_bp) 1) _asplayer_bp)
  (set `/Game/Blueprints/Players/PlayerBP.Points` (+ (`/Game/Blueprints/Players/PlayerBP.Points` _asplayer_bp) 85) _asplayer_bp)
  (bind _asgame_mode_wave_system (cast `/Game/Blueprints/ControllersAndGameModes/GameMode_WaveSystem` (`GameplayStatics.GetGameMode`)))
  (set `/Game/Blueprints/ControllersAndGameModes/GameMode_WaveSystem.EnemyCount` (- (`/Game/Blueprints/ControllersAndGameModes/GameMode_WaveSystem.EnemyCount` _asgame_mode_wave_system) 1) _asgame_mode_wave_system)
  (`self.K2_DestroyActor`) ; Killed
)

(event `self.ReceiveAnyDamage`
  (params (Damage :type "Float (single-precision)") (DamageType :type "DamageType Object Reference") (InstigatedBy :type "Controller Object Reference") (DamageCauser :type "Actor Object Reference"))
  ;[1 1 1] Health (WIP)
)

(fn `DamageOnWave`
  (set `self.EnemyDamage` (+ (`self.Wavedamage`) 10.0)))

(fn `Setstartspeed`
  (set `CharacterMovementComponent.MaxWalkSpeed` (`KismetMathLibrary.RandomFloatInRange` 100.0 200.0) (`self.CharacterMovement`)))

(fn `UpdateEnemySpeed`
  (set `CharacterMovementComponent.MaxWalkSpeed` (+ (`KismetMathLibrary.RandomFloatInRange` 150.0 200.0) (`KismetMathLibrary.RandomFloatInRange` 50.0 90.0)) (`self.CharacterMovement`)))

(fn `UserConstructionScript`)