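; Paper2D side-scroller player character with run, double and wall jump, climbing, dash, health and respawn.
; Tick picks flipbooks through a priority state function, though IsDashing is fed from IsFalling, and flips the sprite by velocity.
; Fire spawns delayed projectiles, while right-stick aiming rotates an arrow that spawns its own.
; Timelines squash the actor on jump and landing; cover is unfinished, and a debug key saves a click counter.
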(event Custom|WallJump
  (bind _returnvalue (Transformation|GetActorForwardVector))
  ;[1 1 1] Wall jump
  (bind (_outhit _returnvalue_2) (Collision|LineTraceByChannel (- (Transformation|GetActorLocation) (* _returnvalue (+ (Components|Capsule|GetScaledCapsuleRadius (Variables|Collision|GetCapsuleComponent)) 15.0))) (+ (Transformation|GetActorLocation) (* _returnvalue (+ (Components|Capsule|GetScaledCapsuleRadius (Variables|Collision|GetCapsuleComponent)) 15.0))) "TraceTypeQuery1" true 0 "None"))
  (if _returnvalue_2
    (Character|LaunchCharacter (Math|Vector|MakeVector (* (Math|Float|Sign(Float) (- (.x (Transformation|GetActorLocation)) (.x (.Location (Collision|BreakHitResult _outhit))))) 4e+02) 0.0 (Variables|/Script/Engine.CharacterMovementComponent|GetJumpZVelocity (Variables|Character|GetCharacterMovement))) true true)
    (CallFunction|JumpFX)
    (elif (<= (Variables|Default|GetJumpCount) 1)
      (Character|Jump)
      (Variables|Default|SetJumpCount (+ (Variables|Default|GetJumpCount) 1))
      (CallFunction|JumpFX))))

(event Custom|LandFX
  ;[1 1 1] JumpFX and LandFX (Squash animation[not animation though])
  (Effects|SpawnEmitteratLocation "/Game/Art/Particles/DustParticle.DustParticle" (Transformation|GetWorldLocation (Variables|Default|GetDustBox)))
  (bind _squash (Timeline|Timeline_1 PlayFromStart)
    (:Update
      (Transformation|SetActorScale3D (Math|Vector|Lerp(Vector) "1.000000,1.000000,1.000000" "1.200000,0.500000,0.200000" _squash)))))

(event Custom|UpdateAnimation
  (bind _charactermovement (Variables|Character|GetCharacterMovement))
  (bind _returnvalue (AI|Components|NavMovement|IsFalling _charactermovement))
  ;[1 1 1] Control Animation
  (Variables|Default|SetIsMoving (> (Math|Vector|VectorLength (Transformation|GetVelocity)) 0.0))
  (bind _outputfb (CallFunction|AnimationStateMaschine (Variables|Default|GetIsMoving) _returnvalue _returnvalue (Variables|Default|GetIsAttacking) (Variables|Default|GetbIsClimbing)))
  (Sprite|SetFlipbook (Variables|Default|GetSprite) _outputfb))

(event Custom|FireProjectile
  ;[1 1 1] Projectile fire and animation (attacking)
  (Game|SpawnActorfromClass "/Game/Blueprints/Projectiles/ProjectileBP1.ProjectileBP1_C" (Transformation|GetWorldTransform (Variables|Default|GetProjectileSpawn)) "AlwaysSpawn" 0 0))

(event Custom|AttackAnimation
  ;[1 1 1] Projectile fire and animation (attacking)
  (Utilities|FlowControl|Sequence
    (:then_0
      (Variables|Default|SetIsAttacking true)
      (Utilities|FlowControl|Delay 0.3)
      (CallFunction|FireProjectile))
    (:then_1
      (Utilities|FlowControl|Delay (/ 5.0 (Variables|/Script/Paper2D.PaperFlipbook|GetFramesPerSecond (Variables|FlipBook|GetAttackFB))))
      (Variables|Default|SetIsAttacking false))))

(event Custom|ClimbingEnd
  ;[1 1 1] Climbing
  (Pawn|Components|CharacterMovement|SetMovementMode (Variables|Character|GetCharacterMovement) "MOVE_Walking" 0)
  (Variables|Default|SetbIsClimbing false)
  (Components|Timeline|SetPlayRate (Variables|Default|GetSprite) 1.0))

(event Custom|TakeCover
  ;[1 1 1] Cover(WIP)
)

(event Custom|JumpFX
  ;[1 1 1] JumpFX and LandFX (Squash animation[not animation though])
  (Effects|SpawnEmitteratLocation "/Game/Art/Particles/DustParticle.DustParticle" (Transformation|GetWorldLocation (Variables|Default|GetDustBox)))
  (bind _squash (Timeline|Timeline_0 PlayFromStart) ; press on the component two times to open the timeline and edit it
    (:Update
      (Transformation|SetActorScale3D (Math|Vector|Lerp(Vector) "1.000000,1.000000,1.000000" "0.250000,1.000000,2.000000" _squash)))))

(event EventIsCoverAvailable
  (params (IsCoverAvailable :type Boolean) (CoverRot :type Rotator :default "0, 0, 0"))
  ;[1 1 1] Cover(WIP)
  (Variables|Default|SetCoverAvailable IsCoverAvailable)
  (Variables|Default|SetCoverRot CoverRot))

(event EventOnLanded
  (params (Hit :type Hit%20Result%20Structure%20%28by%20ref%29))
  ;[1 1 1] Landed
  (Variables|Default|SetJumpCount 0)
  (CallFunction|LandFX))

(event EventTick
  (params (DeltaSeconds :type Float%20%28single-precision%29))
  (bind _sprite (Variables|Default|GetSprite))
  ;[1 1 1] Update (Rotate FlipBook)
  (Variables|Default|SetfDeltaSeconds DeltaSeconds)
  (CallFunction|UpdateAnimation)
  (Math|Float|CompareFloat (.X (Math|Vector|BreakVector (Variables|/Script/Engine.MovementComponent|GetVelocity (Variables|Character|GetCharacterMovement)))) 0.0
    (:>
      (Variables|Default|SetbIsFlipped false)
      (Transformation|SetRelativeRotation _sprite "0, 0, 0" false false))
    (:<
      (Variables|Default|SetbIsFlipped true)
      (Transformation|SetRelativeRotation _sprite "0,180.000000, 0" false false))))

(event Game|Damage|EventAnyDamage
  (params (Damage :type Float%20%28single-precision%29) (DamageType :type Damage%20Type%20Object%20Reference) (InstigatedBy :type Controller%20Object%20Reference) (DamageCauser :type Actor%20Object%20Reference))
  ;[1 1 1] Health
  (Variables|Default|SetHealth (- (Variables|Default|GetHealth) Damage))
  (if (<= (Variables|Default|GetHealth) 0.0)
    (Actor|DestroyActor)))

(event Input|ActionEvents|InputActionJump
  (params (Key :type Key%20Structure))
  ;[1 1 1] Jump and double jump
  (:Pressed
    (if (AI|Components|NavMovement|IsFalling (Variables|Character|GetCharacterMovement))
      (CallFunction|WallJump)
      (else
        (Character|Jump)
        (Variables|Default|SetJumpCount (+ (Variables|Default|GetJumpCount) 1))
        (CallFunction|JumpFX))))
  (:Released
    (Utilities|FlowControl|Delay 0.1)
    (Character|StopJumping)))

(event Input|ActionEvents|InputActionCover
  (params (Key :type Key%20Structure))
  ;[1 1 1] Cover(WIP)
  (:Pressed
    (CallFunction|TakeCover (stale _asplayer_bp))))

(event Input|ActionEvents|InputActionFire
  (params (Key :type Key%20Structure))
  ;[1 1 1] Projectile fire and animation (attacking)
  (:Pressed
    (if (not (Variables|Default|GetIsAttacking))
      (CallFunction|AttackAnimation))))

(event Input|ActionEvents|InputActionDash
  (params (Key :type Key%20Structure))
  (bind _returnvalue (Transformation|GetVelocity))
  ;[1 1 1] Dash
  (:Pressed
    (if (Math|Vector|NotEqual(Vector) _returnvalue "0, 0, 0" 0.0001)
      (if (AI|Components|NavMovement|IsFalling (Variables|Character|GetCharacterMovement))
        (Character|LaunchCharacter (* (+ _returnvalue "0, 0, 0") "0, 0, 0") true true)
        (else
          (Character|LaunchCharacter (* (+ _returnvalue "0.500000,0.500000,0.500000") "1.500000,1.000000,150.000000") true true))))))

(event Input|AxisEvents|InputAxisRight
  (params (AxisValue :type Float%20%28single-precision%29))
  ;[1 1 1] movement
  (Pawn|Input|AddMovementInput "1.000000, 0, 0" AxisValue false))

(event Input|AxisEvents|InputAxisUp
  (params (AxisValue :type Float%20%28single-precision%29))
  ;[1 1 1] Climbing
  (if (Variables|Default|GetbCanClimb)
    (if (Math|Float|InRange(Float) AxisValue -0.1 0.1)
      (Components|Timeline|SetPlayRate (Variables|Default|GetSprite) 0.0)
      (else
        (Variables|Default|SetbIsClimbing true)
        (Components|Timeline|SetPlayRate (Variables|Default|GetSprite) 1.0)
        (Pawn|Components|CharacterMovement|SetMovementMode (Variables|Character|GetCharacterMovement) "MOVE_Flying" 0)
        (Pawn|Input|AddMovementInput "0, 0,0.500000" AxisValue false)))))

(event Input|GamepadEvents|GamepadRightX
  (params (AxisValue :type Float%20%28single-precision%29))
  (bind _returnvalue (Transformation|GetActorLocation))
  (bind _arrowshooting (Variables|Default|GetArrowShooting))
  (bind _arrowshooting_2 (Variables|Default|GetArrowShooting))
  ;[1 1 1] Aiming / Shooting Controller
  (if (or (> AxisValue 0.5) (< AxisValue -0.5))
    (bind _output_get (Variables|Default|SetbIsShootingY true))
    (bind _output_get_2 (Variables|Default|SetbIsShootingX true))
    ;;[1 1 1] Tick
    (Variables|Default|SetfDeltaSeconds (Variables|Default|GetfDeltaSeconds))
    (if (Variables|Default|GetbIsFlipped)
      ;;[1 1 1] 180° left aiming
      (Transformation|SetRelativeRotation _arrowshooting (Math|Rotator|MakeRotator (.Roll (Math|Rotator|BreakRotator (Math|Rotator|FindLookatRotation _returnvalue (+ _returnvalue (Math|Vector|MakeVector AxisValue 0.0 (* (stale Input|GamepadEvents|GamepadRightY AxisValue) -1.0)))))) (Math|Float|ClampAngle (.Pitch (Math|Rotator|BreakRotator (Math|Rotator|FindLookatRotation _returnvalue (+ _returnvalue (Math|Vector|MakeVector AxisValue 0.0 (* (stale Input|GamepadEvents|GamepadRightY AxisValue) -1.0)))))) -9e+01 9e+01) (- (Math|Float|ClampAngle (- (.Yaw (Math|Rotator|BreakRotator (Math|Rotator|FindLookatRotation _returnvalue (+ _returnvalue (Math|Vector|MakeVector AxisValue 0.0 (* (stale Input|GamepadEvents|GamepadRightY AxisValue) -1.0)))))) 1.8e+02) 0.0 0.0) 1.8e+02)) false false)
      (if (or (Variables|Default|GetbIsShootingY) (Variables|Default|GetbIsShootingX))
        (Utilities|FlowControl|Delay (Variables|Default|GetfProjectileDelay))
        (Game|SpawnActorfromClass "/Game/Blueprints/Projectiles/ProjectilePlayer_BP.ProjectilePlayer_BP_C" (Transformation|GetWorldTransform _arrowshooting) "Undefined" 0 0))
      (else
        ;;[1 1 1] 180° right aiming
        (Transformation|SetRelativeRotation _arrowshooting_2 (Math|Rotator|MakeRotator (.Roll (Math|Rotator|BreakRotator (Math|Rotator|FindLookatRotation _returnvalue (+ _returnvalue (Math|Vector|MakeVector AxisValue 0.0 (* (stale Input|GamepadEvents|GamepadRightY AxisValue) -1.0)))))) (Math|Float|ClampAngle (.Pitch (Math|Rotator|BreakRotator (Math|Rotator|FindLookatRotation _returnvalue (+ _returnvalue (Math|Vector|MakeVector AxisValue 0.0 (* (stale Input|GamepadEvents|GamepadRightY AxisValue) -1.0)))))) -9e+01 9e+01) (+ (Math|Float|ClampAngle (- (.Yaw (Math|Rotator|BreakRotator (Math|Rotator|FindLookatRotation _returnvalue (+ _returnvalue (Math|Vector|MakeVector AxisValue 0.0 (* (stale Input|GamepadEvents|GamepadRightY AxisValue) -1.0)))))) 0.0) 0.0 0.0) 0.0)) false false)
        (if (or (Variables|Default|GetbIsShootingY) (Variables|Default|GetbIsShootingX))
          (Utilities|FlowControl|Delay (Variables|Default|GetfProjectileDelay))
          (Game|SpawnActorfromClass "/Game/Blueprints/Projectiles/ProjectilePlayer_BP.ProjectilePlayer_BP_C" (Transformation|GetWorldTransform _arrowshooting_2) "Undefined" 0 0))))
    (else
      (bind _output_get_3 (Variables|Default|SetbIsShootingX false)))))

(event Input|GamepadEvents|GamepadRightY
  (params (AxisValue :type Float%20%28single-precision%29))
  (bind _returnvalue (Transformation|GetActorLocation))
  (bind _arrowshooting (Variables|Default|GetArrowShooting))
  (bind _arrowshooting_2 (Variables|Default|GetArrowShooting))
  ;[1 1 1] Aiming / Shooting Controller
  (if (or (> AxisValue 0.5) (< AxisValue 0.0))
    (bind _output_get (Variables|Default|SetbIsShootingY true))
    (bind _output_get_2 (Variables|Default|SetbIsShootingX true))
    ;;[1 1 1] Tick
    (Variables|Default|SetfDeltaSeconds (Variables|Default|GetfDeltaSeconds))
    (if (Variables|Default|GetbIsFlipped)
      ;;[1 1 1] 180° left aiming
      (Transformation|SetRelativeRotation _arrowshooting (Math|Rotator|MakeRotator (.Roll (Math|Rotator|BreakRotator (Math|Rotator|FindLookatRotation _returnvalue (+ _returnvalue (Math|Vector|MakeVector (stale Input|GamepadEvents|GamepadRightX AxisValue) 0.0 (* AxisValue -1.0)))))) (Math|Float|ClampAngle (.Pitch (Math|Rotator|BreakRotator (Math|Rotator|FindLookatRotation _returnvalue (+ _returnvalue (Math|Vector|MakeVector (stale Input|GamepadEvents|GamepadRightX AxisValue) 0.0 (* AxisValue -1.0)))))) -9e+01 9e+01) (- (Math|Float|ClampAngle (- (.Yaw (Math|Rotator|BreakRotator (Math|Rotator|FindLookatRotation _returnvalue (+ _returnvalue (Math|Vector|MakeVector (stale Input|GamepadEvents|GamepadRightX AxisValue) 0.0 (* AxisValue -1.0)))))) 1.8e+02) 0.0 0.0) 1.8e+02)) false false)
      (if (or (Variables|Default|GetbIsShootingY) (Variables|Default|GetbIsShootingX))
        (Utilities|FlowControl|Delay (Variables|Default|GetfProjectileDelay))
        (Game|SpawnActorfromClass "/Game/Blueprints/Projectiles/ProjectilePlayer_BP.ProjectilePlayer_BP_C" (Transformation|GetWorldTransform _arrowshooting) "Undefined" 0 0))
      (else
        ;;[1 1 1] 180° right aiming
        (Transformation|SetRelativeRotation _arrowshooting_2 (Math|Rotator|MakeRotator (.Roll (Math|Rotator|BreakRotator (Math|Rotator|FindLookatRotation _returnvalue (+ _returnvalue (Math|Vector|MakeVector (stale Input|GamepadEvents|GamepadRightX AxisValue) 0.0 (* AxisValue -1.0)))))) (Math|Float|ClampAngle (.Pitch (Math|Rotator|BreakRotator (Math|Rotator|FindLookatRotation _returnvalue (+ _returnvalue (Math|Vector|MakeVector (stale Input|GamepadEvents|GamepadRightX AxisValue) 0.0 (* AxisValue -1.0)))))) -9e+01 9e+01) (+ (Math|Float|ClampAngle (- (.Yaw (Math|Rotator|BreakRotator (Math|Rotator|FindLookatRotation _returnvalue (+ _returnvalue (Math|Vector|MakeVector (stale Input|GamepadEvents|GamepadRightX AxisValue) 0.0 (* AxisValue -1.0)))))) 0.0) 0.0 0.0) 0.0)) false false)
        (if (or (Variables|Default|GetbIsShootingY) (Variables|Default|GetbIsShootingX))
          (Utilities|FlowControl|Delay (Variables|Default|GetfProjectileDelay))
          (Game|SpawnActorfromClass "/Game/Blueprints/Projectiles/ProjectilePlayer_BP.ProjectilePlayer_BP_C" (Transformation|GetWorldTransform _arrowshooting_2) "Undefined" 0 0))))
    (else
      (bind _output_get_3 (Variables|Default|SetbIsShootingY false)))))

(event Input|KeyboardEvents|C
  (params (Key :type Key%20Structure))
  ;[1 1 1] Save Data
  (:Pressed
    (bind _returnvalue (SaveGame|DoesSaveGameExist "SlotName"))
    (if _returnvalue
      (bind _returnvalue_2 (SaveGame|LoadGamefromSlot "SlotName"))
      (bind _output_get (Variables|Default|SetSaverSubClass _returnvalue_2)) ; Store the info
      (bind _asmy_save_game (Utilities|Casting|CastToMySaveGame _output_get))
      (bind _result (Math|Integer|IncrementInt (Variables|/Game/Blueprints/Interface/MySaveGame.MySaveGame_C|GetNumberOfClicks _asmy_save_game))
        (:%20%20
          (SaveGame|SaveGametoSlot (Variables|Default|GetSaverSubClass) "SlotName")
          (Development|PrintString (Utilities|String|ToString(Integer) _result))))
      (else
        (bind _returnvalue_3 (SaveGame|CreateSaveGameObject "/Game/Blueprints/Interface/MySaveGame.MySaveGame_C"))
        (bind _output_get_2 (Variables|Default|SetSaverSubClass _returnvalue_3)) ; create save of the info
        (bind _asmy_save_game_2 (Utilities|Casting|CastToMySaveGame _output_get_2))
        (bind _result_2 (Math|Integer|IncrementInt (Variables|/Game/Blueprints/Interface/MySaveGame.MySaveGame_C|GetNumberOfClicks _asmy_save_game_2))
          (:%20%20
            (SaveGame|SaveGametoSlot (Variables|Default|GetSaverSubClass) "SlotName")
            (Development|PrintString (Utilities|String|ToString(Integer) _result_2))))))))

(event Input|KeyboardEvents|T
  (params (Key :type Key%20Structure))
  ;[1 1 1] transform to checkpoint
  (:Pressed
    (Actor|DestroyActor)
    (CallFunction|RespawnPlayer (Variables|Default|GetSpawntransform))))

(fn ConstructionScript
  ;[1 1 1] Holding jump
  (Variables|/Script/Engine.CharacterMovementComponent|SetJumpZVelocity (Variables|Character|GetCharacterMovement) 3.5e+02)
  (Variables|Default|SetJumpMaxHoldTime 0.2)
  (Variables|Default|SetJumpCount 0)
  ;[1 1 1] Health
  (Variables|Default|SetHealth (Variables|Default|GetMaxHealth)))

(fn AnimationStateMaschine
  (params (bIsMoving :type Boolean) (bIsFalling :type Boolean) (bIsDashing :type Boolean) (bIsAttacking :type Boolean) (bIsClimbing :type Boolean))
  (if bIsClimbing
    (LocalVariables|SetAnimationState "NewEnumerator5")
    (elif bIsDashing
      (LocalVariables|SetAnimationState "NewEnumerator3")
      (elif bIsAttacking
        (LocalVariables|SetAnimationState "NewEnumerator4")
        (elif bIsFalling
          (LocalVariables|SetAnimationState "NewEnumerator2")
          (elif bIsMoving
            (LocalVariables|SetAnimationState "NewEnumerator1")
            (else
              (LocalVariables|SetAnimationState "NewEnumerator0")))))))
  (return (Utilities|Select :Index (LocalVariables|GetAnimationState) :NewEnumerator0 (Variables|FlipBook|GetIdleFB) :NewEnumerator1 (Variables|FlipBook|GetRunningFB) :NewEnumerator2 (Variables|FlipBook|GetJumpingFB) :NewEnumerator3 (Variables|FlipBook|GetDashingFB) :NewEnumerator4 (Variables|FlipBook|GetAttackFB) :NewEnumerator5 (Variables|FlipBook|GetClimbing))))

(fn RespawnPlayer
  (params (Spawntransform :type Transform))
  (bind _returnvalue (Game|SpawnActorfromClass "/Game/Blueprints/Players/PlayerBP.PlayerBP_C" Spawntransform "Undefined" 0 0))
  (Pawn|Possess (Game|GetPlayerController 0) _returnvalue))