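; Player character for a 2D side-scroller with running, jumping, dashing and twin-stick shooting.
; Jump input jumps from the ground; in the air, a forward-axis line trace triggers a wall kick or falls back to a count-limited extra jump.
; Movement flips the replicated sprite and picks idle, run or jump flipbooks through a macro-style state machine.
; Tick aims an arrow by gamepad stick, clamped to the facing side, and spawns delay-throttled BP_Bullet actors.
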(event `self.OnLanded`
  (params (Hit :type "HitResult Structure (by ref)"))
  ;[1 1 1] landed
  (set `self.JumpCount` 0))

(event `self.ReceiveBeginPlay`
  ;[1 1 1] Replication
  (`ActorComponent.SetIsReplicated` (`self.Sprite`) true))

(event `InputAction|Jump`
  (params (Key :type "Key Structure"))
  ;[1 1 1] ControllerJump
  (:`Pressed`
    (if (> (stale `InputAxisKey|Gamepad_LeftY` AxisValue) 0.65)
      (if (`NavMovementComponent.IsFalling` (`self.CharacterMovement`))
        (`self.WallJump`)
        (else
          (`self.Jump`)
          (set `self.JumpCount` (+ (`self.JumpCount`) 1)))))))

(event `InputAction|Jump`
  (params (Key :type "Key Structure"))
  ;[1 1 1] KeyboardJump
  (:`Pressed`
    (if (`NavMovementComponent.IsFalling` (`self.CharacterMovement`))
      (`self.WallJump`)
      (else
        (`self.Jump`)
        (set `self.JumpCount` (+ (`self.JumpCount`) 1)))))
  (:`Released`
    (`self.StopJumping`)))

(event `InputAction|Dash`
  (params (Key :type "Key Structure"))
  (bind _returnvalue (`self.GetVelocity`))
  ;[1 1 1] Dash
  (:`Pressed`
    (if (!= _returnvalue (0.0 0.0 0.0))
      (if (`NavMovementComponent.IsFalling` (`self.CharacterMovement`))
        (`self.LaunchCharacter` (* (+ _returnvalue (0.0 0.0 0.0)) (2.0 2.0 2.0)) true true)
        (else
          (`self.LaunchCharacter` (* (+ _returnvalue (0.0 0.0 1.0)) (1.5 1.5 250.0)) true true))))))

(event `InputAxisKey|Gamepad_LeftY`
  (params (AxisValue :type "Float (single-precision)"))
  ;[1 1 1] ControllerJump
)

(event `InputAxis|MoveRight`
  (params (AxisValue :type "Float (single-precision)"))
  (bind _sprite (`self.Sprite`))
  ;[1 1 1] Movement
  (`self.AddMovementInput` (1.0 0.0 0.0) AxisValue)
  (`self.UpdateAnimation`)
  (`/Engine/EditorBlueprintResources/StandardMacros.CompareFloat` AxisValue
    (:`>`
      (set `self.bIsFlipped` false)
      (`SceneComponent.K2_SetRelativeRotation` :`self` _sprite))
    (:`<`
      (set `self.bIsFlipped` true)
      (`SceneComponent.K2_SetRelativeRotation` _sprite (struct :`Yaw` 180.0) false false))))

(event `UpdateAnimation`
  ;[1 1 1] Animation Handling
  (set `self.IsMoving` (> (`KismetMathLibrary.VSize` (`self.GetVelocity`)) 0.0))
  (set `self.IsFalling` (`NavMovementComponent.IsFalling` (`self.CharacterMovement`)))
  (bind _outputflipbook (`self.AnimationStateMachine` (`self.IsFalling`) (`self.IsMoving`)))
  (`PaperFlipbookComponent.SetFlipbook` (`self.Sprite`) _outputflipbook))

(event `InputAxisKey|Gamepad_RightY`
  (params (AxisValue :type "Float (single-precision)"))
  ;[1 1 1] Aiming / Shooting
  (if (or (> AxisValue 0.5) (< AxisValue 0.0))
    (bind _output_get (set `self.bIsShootingY` true :!label _label))
    (bind _output_get_2 (set `self.bIsShootingX` true))
    (else
      (bind _output_get_3 (set `self.bIsShootingY` false)))))

(event `InputAxisKey|Gamepad_RightX`
  (params (AxisValue :type "Float (single-precision)"))
  ;[1 1 1] Aiming / Shooting
  (if (or (> AxisValue 0.5) (< AxisValue -0.5))
    (goto _label)
    (else
      (bind _output_get (set `self.bIsShootingX` false)))))

(event `self.ReceiveTick`
  (params (DeltaSeconds :type "Float (single-precision)"))
  (bind _returnvalue (`self.K2_GetActorLocation`))
  (bind _arrowshooting (`self.ArrowShooting`))
  (bind _arrowshooting_2 (`self.ArrowShooting`))
  ;[1 1 1] Aiming / Shooting
  ;;[1 1 1] Tick
  (set `self.fDeltaSeconds` DeltaSeconds)
  (if (`self.bIsFlipped`)
    (bind _returnvalue_2 (`KismetMathLibrary.FindLookAtRotation` _returnvalue (+ _returnvalue (`KismetMathLibrary.MakeVector` (stale `InputAxisKey|Gamepad_RightX` AxisValue) 0.0 (* (stale `InputAxisKey|Gamepad_RightY` AxisValue) -1.0)))))
    ;;[1 1 1] 180° left aiming
    (`SceneComponent.K2_SetRelativeRotation` _arrowshooting (`KismetMathLibrary.MakeRotator` (.roll _returnvalue_2) (`KismetMathLibrary.ClampAngle` (.pitch _returnvalue_2) -90.0 90.0) (- (`KismetMathLibrary.ClampAngle` (- (.yaw _returnvalue_2) 180.0)) 180.0)) false false)
    (if (or (`self.bIsShootingY`) (`self.bIsShootingX`))
      (`KismetSystemLibrary.Delay` (`self.fProjectileDelay`))
      (`|SpawnActorFromClass` "/Game/Blueprints/Projectiles/BP_Bullet.BP_Bullet_C" (`SceneComponent.K2_GetComponentToWorld` _arrowshooting) "Undefined" "OverrideRootScale" null null))
    (else
      ;;[1 1 1] 180° right aiming
      (`SceneComponent.K2_SetRelativeRotation` _arrowshooting_2 (`KismetMathLibrary.MakeRotator` (.roll _returnvalue_2) (`KismetMathLibrary.ClampAngle` (.pitch _returnvalue_2) -90.0 90.0) (+ (`KismetMathLibrary.ClampAngle` (- (.yaw _returnvalue_2) 0.0)) 0.0)) false false)
      (if (or (`self.bIsShootingY`) (`self.bIsShootingX`))
        (`KismetSystemLibrary.Delay` (`self.fProjectileDelay`))
        (`|SpawnActorFromClass` "/Game/Blueprints/Projectiles/BP_Bullet.BP_Bullet_C" (`SceneComponent.K2_GetComponentToWorld` _arrowshooting_2) "Undefined" "OverrideRootScale" null null)))))

(event `WallJump`
  (bind _returnvalue_x (`KismetMathLibrary.BreakVector` (`self.K2_GetActorLocation`)))
  (bind _returnvalue (`self.GetActorForwardVector`))
  (bind (_outhit _returnvalue_2) (`KismetSystemLibrary.LineTraceSingle` (- (`self.K2_GetActorLocation`) (* _returnvalue (+ (`CapsuleComponent.GetScaledCapsuleRadius` (`self.CapsuleComponent`)) 15.0))) (+ (`self.K2_GetActorLocation`) (* _returnvalue (+ (`CapsuleComponent.GetScaledCapsuleRadius` (`self.CapsuleComponent`)) 15.0))) "TraceTypeQuery1" true))
  (if _returnvalue_2
    (`self.LaunchCharacter` (`KismetMathLibrary.MakeVector` (* (`KismetMathLibrary.SignOfFloat` (- _returnvalue_x (.x (`.Location` (`GameplayStatics.BreakHitResult` _outhit))))) 450.0) 0.0 (`CharacterMovementComponent.JumpZVelocity` (`self.CharacterMovement`))) true true)
    (elif (<= (`self.JumpCount`) 1)
      (`self.Jump`)
      (set `self.JumpCount` (+ (`self.JumpCount`) 1)))))

(fn `AnimationStateMachine`
  (params (IsFalling :type Boolean) (IsMoving :type Boolean))
  (returns (OutputFlipbook :type "PaperFlipbook Object Reference"))
  (locals (AnimationState :type "/Game/Data_Enums/Enum_AnimationState Enum") (IsFallingLocal :type Boolean) (IsMovingLocal :type Boolean))
  ;[1 1 1] Collect Data
  (set `local.IsFallingLocal` IsFalling)
  (set `local.IsMovingLocal` IsMoving)
  ;[1 1 1] Test Data
  (if (`local.IsFallingLocal`)
    ;[1 1 1] Set Animation State
    (set `local.AnimationState` "NewEnumerator2")
    (elif (`local.IsMovingLocal`)
      (set `local.AnimationState` "NewEnumerator1")
      (else
        (set `local.AnimationState` "NewEnumerator0"))))
  (return (select `/Game/Data_Enums/Enum_AnimationState` (`local.AnimationState`) :`NewEnumerator0` (`self.IdleFlipbook`) :`NewEnumerator1` (`self.RunFlipbook`) :`NewEnumerator2` (`self.JumpFlipbook`))))

(fn `UserConstructionScript`
  (set `CharacterMovementComponent.JumpZVelocity` 400.0 (`self.CharacterMovement`))
  (set `self.JumpMaxHoldTime` 0.2)
  (set `self.JumpCount` 0))