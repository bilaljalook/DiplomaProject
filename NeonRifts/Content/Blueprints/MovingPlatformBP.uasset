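; Moving platform actor that travels between its starting location and an offset from it.
; On BeginPlay it stores its location as StartPos and plays MovementTimeline from the start.
; Each timeline update lerps the position toward StartPos plus Speed using the Movement track as alpha, so Speed acts as a travel offset rather than a velocity.
; The location is set without sweep, so movement ignores blocking collision.
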(event `self.ReceiveBeginPlay`
  (bind (_startpos_x _startpos_y _startpos_z) (`KismetMathLibrary.BreakVector` (`self.StartPos`)))
  (bind (_speed_x _speed_y _speed_z) (`KismetMathLibrary.BreakVector` (`self.Speed`)))
  (set `self.StartPos` (`self.K2_GetActorLocation`))
  (bind (_direction _movement) (`Timeline|MovementTimeline` :!via `PlayFromStart`)
    (:`Update`
      (`self.K2_SetActorLocation` (`KismetMathLibrary.VLerp` (`self.StartPos`) (`KismetMathLibrary.MakeVector` (+ _startpos_x _speed_x) (+ _startpos_y _speed_y) (+ _startpos_z _speed_z)) _movement)))))

(fn `UserConstructionScript`)