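; Behavior tree service that copies enemy AI state from the controlled Enemy_AI_BP pawn into the blackboard.
; Each tick, it updates the CombatStatus key whenever it differs from the pawn's value.
; DoOnce gates write the PlayerCharacter key a single time once that reference passes its check, and the CombatType key on the first tick only.
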(event `self.ReceiveTickAI`
  (params (OwnerController :type "AIController Object Reference") (ControlledPawn :type "Pawn Object Reference") (DeltaSeconds :type "Float (single-precision)"))
  (bind _combatstatus (`self.CombatStatus`))
  (bind _asenemy_ai_bp (cast `/Game/Blueprints/Players/Enemy_AI_BP` ControlledPawn))
  (`|ExecutionSequence`
    (:`then_0`
      (bind _combatstatus_2 (`/Game/Blueprints/Players/Enemy_AI_BP.CombatStatus` _asenemy_ai_bp))
      (if (not (== (`BTFunctionLibrary.GetBlackboardValueAsEnum` _combatstatus) _combatstatus_2))
        (`BTFunctionLibrary.SetBlackboardValueAsEnum` _combatstatus _combatstatus_2)))
    (:`then_1`
      (bind _playercharacter (`/Game/Blueprints/Players/Enemy_AI_BP.PlayerCharacter` _asenemy_ai_bp))
      (if (not (== _playercharacter null))
        (`/Engine/EditorBlueprintResources/StandardMacros.DoOnce` false
          (:`Completed`
            (`BTFunctionLibrary.SetBlackboardValueAsObject` (`self.PlayerCharacter`) _playercharacter)))))
    (:`then_2`
      (`/Engine/EditorBlueprintResources/StandardMacros.DoOnce` false
        (:`Completed`
          (`BTFunctionLibrary.SetBlackboardValueAsEnum` (`self.CombatType`) (`/Game/Blueprints/Players/Enemy_AI_BP.CombatType` _asenemy_ai_bp)))))))