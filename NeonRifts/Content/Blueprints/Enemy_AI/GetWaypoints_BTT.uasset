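; GetWaypoints_BTT is a behavior tree task that copies an enemy's two patrol waypoints into the blackboard.
; On first execution it casts the controlled pawn to Enemy_AI_BP and writes its Waypoint1 and Waypoint2 vectors to blackboard keys.
; A WaypointsSet flag makes later executions succeed immediately without writing again.
; A failed cast stops the graph without finishing the task.
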(event `self.ReceiveExecuteAI`
  (params (OwnerController :type "AIController Object Reference") (ControlledPawn :type "Pawn Object Reference"))
  (if (`self.WaypointsSet`)
    (`self.FinishExecute` true)
    (else
      (bind _asenemy_ai_bp (cast `/Game/Blueprints/Players/Enemy_AI_BP` ControlledPawn))
      (`BTFunctionLibrary.SetBlackboardValueAsVector` (`self.Waypoint1`) (`/Game/Blueprints/Players/Enemy_AI_BP.Waypoint1` _asenemy_ai_bp))
      (`BTFunctionLibrary.SetBlackboardValueAsVector` (`self.Waypoint2`) (`/Game/Blueprints/Players/Enemy_AI_BP.Waypoint2` _asenemy_ai_bp))
      (set `self.WaypointsSet` true)
      (`self.FinishExecute` true))))