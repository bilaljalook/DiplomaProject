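; Behavior Tree decorator for enemy AI that checks whether the controlled pawn is within a threshold distance of the player.
; It compares the pawn's location with that of the PlayerCharacter blackboard actor.
; As a side effect, it clears that blackboard key when player 0's PlayerBP has zero Health, before the distance is read.
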(fn `PerformConditionCheckAI`
  (params (OwnerController :type "AIController Object Reference") (ControlledPawn :type "Pawn Object Reference"))
  (returns (ReturnValue :type Boolean))
  (bind _asplayer_bp (cast `/Game/Blueprints/Players/PlayerBP` (`GameplayStatics.GetPlayerPawn` 0)))
  (if (== (`/Game/Blueprints/Players/PlayerBP.Health` _asplayer_bp) 0.0)
    (`BTFunctionLibrary.ClearBlackboardValue` (`self.PlayerCharacter`)))
  (return (< (`KismetMathLibrary.VSize` (- (`Actor.K2_GetActorLocation` ControlledPawn) (`Actor.K2_GetActorLocation` (`BTFunctionLibrary.GetBlackboardValueAsActor` (`self.PlayerCharacter`))))) (`self.DistanceThreshhold`))))